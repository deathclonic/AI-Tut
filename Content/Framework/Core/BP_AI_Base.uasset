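; Base AI character that provides player sensing, targeting and death handling, with an empty behavior event.
; While enabled, server-side Tick fires that event, throttled by a DoN and short delay.
; Sense functions track detected and seen players, sight line-traces from the eyes to player mesh sockets, and nearest-player lookup compares navigation path costs rather than straight-line distance.
; Death stops behavior and movement, ragdolls the mesh and disables capsule collision.
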(event `self.ReceiveTick`
  (params (DeltaSeconds :type "Float (single-precision)"))
  (`/Engine/EditorBlueprintResources/ActorMacros.Switch Has Authority`
    (:`Authority`
      (`self.ParentTick` DeltaSeconds)
      (if (`self.EnableBehavior`)
        (`/Engine/EditorBlueprintResources/StandardMacros.Do N` 1 :!label _label
          (:`Exit`
            (`|ExecutionSequence`
              (:`then_0`
                (`self.S_RunBehavior`))
              (:`then_1`
                (`KismetSystemLibrary.Delay` 0.2)
                (goto _label :!via `Reset`)))))))))

(event `S_RunBehavior`)

(event `ParentTick`
  (params (DeltaSeconds :type "Float (double-precision)")))

(event `Death`
  (bind _mesh (`self.Mesh`))
  (set `self.EnableBehavior` false)
  (`MovementComponent.StopMovementImmediately` (`self.CharacterMovement`))
  (`SkeletalMeshComponent.SetAllBodiesSimulatePhysics` _mesh true)
  (`SkeletalMeshComponent.SetAllBodiesPhysicsBlendWeight` _mesh 1.0 false)
  (`PrimitiveComponent.SetCollisionEnabled` (`self.CapsuleComponent`) "NoCollision"))

(fn `GetNearestPlayer`
  (params (UseSenses :type Boolean) (SenseSelection :type "/Game/Framework/Blueprints/AI/E_Senses Enum" :default "NewEnumerator0"))
  (returns (TargetPlayer :type "/Game/Framework/Blueprints/AI/BP_Player Object Reference"))
  (locals (L_TargetPlayer :type "Array of /Game/Framework/Blueprints/AI/BP_Player Object Reference") (L_TargetPlayerDistance :type "Array of Float (double-precision)"))
  (if UseSenses
    (switch `/Game/Framework/Blueprints/AI/E_Senses` SenseSelection
      (:`NewEnumerator0`
        ;[1 1 1] Which player is closest in detection radius
        (`KismetArrayLibrary.Array_Clear` (`local.L_TargetPlayer`))
        (`KismetArrayLibrary.Array_Clear` (`local.L_TargetPlayerDistance`))
        (for _array_element (`self.DetectedPlayers`)
          (`KismetArrayLibrary.Array_Add` (`local.L_TargetPlayer`) _array_element)
          (`KismetArrayLibrary.Array_Add` (`local.L_TargetPlayerDistance`) (`NavigationSystemV1.GetPathCost` (`self.GetLocation`) (`self.GetLocation` _array_element) null "/Script/NavigationSystem.NavigationQueryFilter")))
        (return (`|GetArrayItem` (`local.L_TargetPlayer`) (`KismetMathLibrary.MinOfFloatArray` (`local.L_TargetPlayerDistance`)))))
      (:`NewEnumerator1`
        ;[1 1 1] Which player is closest in sight
        (`KismetArrayLibrary.Array_Clear` (`local.L_TargetPlayer`))
        (`KismetArrayLibrary.Array_Clear` (`local.L_TargetPlayerDistance`))
        (for _array_element_2 (`self.SeenPlayers`)
          (`KismetArrayLibrary.Array_Add` (`local.L_TargetPlayer`) _array_element_2)
          (`KismetArrayLibrary.Array_Add` (`local.L_TargetPlayerDistance`) (`NavigationSystemV1.GetPathCost` (`self.GetLocation`) (`self.GetLocation` _array_element_2) null "/Script/NavigationSystem.NavigationQueryFilter")))
        (return (`|GetArrayItem` (`local.L_TargetPlayer`) (`KismetMathLibrary.MinOfFloatArray` (`local.L_TargetPlayerDistance`))))))
    (else
      ;[1 1 1] Grab all player actors and measure which is closest
      (`KismetArrayLibrary.Array_Clear` (`local.L_TargetPlayer`))
      (`KismetArrayLibrary.Array_Clear` (`local.L_TargetPlayerDistance`))
      (bind _outactors (`GameplayStatics.GetAllActorsOfClass` "/Game/Framework/Blueprints/AI/BP_Player.BP_Player_C"))
      (for _array_element_3 _outactors
        (`KismetArrayLibrary.Array_Add` (`local.L_TargetPlayer`) _array_element_3)
        (`KismetArrayLibrary.Array_Add` (`local.L_TargetPlayerDistance`) (`NavigationSystemV1.GetPathCost` (`self.GetLocation`) (`self.GetLocation` _array_element_3) null "/Script/NavigationSystem.NavigationQueryFilter")))
      (return (`|GetArrayItem` (`local.L_TargetPlayer`) (`KismetMathLibrary.MinOfFloatArray` (`local.L_TargetPlayerDistance`)))))))

(fn `PlayerSensed`
  (params (Selection :type "/Game/Framework/Blueprints/AI/E_Senses Enum" :default "NewEnumerator0") (Player :type "/Game/Framework/Blueprints/AI/BP_Player Object Reference"))
  (switch `/Game/Framework/Blueprints/AI/E_Senses` Selection
    (:`NewEnumerator0`
      (if (`self.IsChasingAPlayer`)
        (bind _output_get (set `self.NewPlayer` Player))
        (`KismetArrayLibrary.Array_Add` (`self.DetectedPlayers`) _output_get)
        (else
          (bind _output_get_2 (set `self.NearestPlayer` Player))
          (`KismetArrayLibrary.Array_Add` (`self.DetectedPlayers`) _output_get_2)
          (set `self.PlayerDetected` true)
          (set `self.IsChasingAPlayer` true))))
    (:`NewEnumerator1`
      (if (`self.IsChasingAPlayer`)
        ;[1 1 1] Add new players to the detected array
        (bind _output_get_3 (set `self.NewPlayer` Player))
        (`KismetArrayLibrary.Array_Add` (`self.SeenPlayers`) _output_get_3)
        (else
          ;[1 1 1] If not currently chasing a player, set as detected player
          (bind _output_get_4 (set `self.SeenPlayer` Player))
          (`KismetArrayLibrary.Array_Add` (`self.SeenPlayers`) _output_get_4)
          (set `self.PlayerDetected` true)
          (set `self.IsChasingAPlayer` true))))))

(fn `PlayerUnsensed`
  (params (Selection :type "/Game/Framework/Blueprints/AI/E_Senses Enum" :default "NewEnumerator0") (Player :type "/Game/Framework/Blueprints/AI/BP_Player Object Reference (by ref)"))
  (switch `/Game/Framework/Blueprints/AI/E_Senses` Selection
    (:`NewEnumerator0`
      (`KismetArrayLibrary.Array_RemoveItem` (`self.DetectedPlayers`) Player))
    (:`NewEnumerator1`
      (`KismetArrayLibrary.Array_RemoveItem` (`self.SeenPlayers`) Player))))

(fn `SightPerception`
  ;[1 1 1] Check if the player is in sight based on the array of sockets in the mesh
  (`self.SeenPlayer`
    (:`then`
      (set `self.PlayerCurrentlyInSight` false)
      (for _array_element (`self.PlayerMeshSockets`)
        (bind _outhit (`KismetSystemLibrary.LineTraceSingle` (`SceneComponent.K2_GetComponentLocation` (`self.Eyes`)) (`SceneComponent.GetSocketLocation` (`Character.Mesh` (`self.SeenPlayer`)) _array_element) "TraceTypeQuery1" false (`|MakeArray` self :!type "Actor Object Reference")))
        (if (`GameplayStatics.BreakHitResult` _outhit)
          (bind _asbp_player (cast `/Game/Framework/Blueprints/AI/BP_Player` (`.HitActor` (`GameplayStatics.BreakHitResult` _outhit))))
          (bind _output_get (set `self.SeenPlayer` _asbp_player))
          (set `self.LastSeenLocation` (`self.GetLocation` _output_get))
          (set `self.bPlayerSeen` true)
          (set `self.PlayerCurrentlyInSight` true)
          (break)))
      (return))
    (:`else`
      (return))))

(fn `UserConstructionScript`
  (`parent.UserConstructionScript`))