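; Simple AI character that runs from players to hiding spots chosen by the EQS_HideFromPlayer query.
; Sight and detection trigger volumes register players, with detection overlap switching behavior from sight checks to a line-of-sight trace.
; A visible player reruns the query, also run at BeginPlay, and the AI sprints to the first result.
; Without a sensed player it stops and resets speed; wall-aware wander logic exists but SRunBehavior never calls it.
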(event `self.S_RunBehavior`
  (if (`self.UseSight`)
    (bind _targetplayer (`self.GetNearestPlayer` true "NewEnumerator1"))
    (set `self.SeenPlayer` _targetplayer)
    (`self.SightPerception`)
    (if (`self.PlayerCurrentlyInSight`)
      (`self.UpdateEQS`)
      (else
        (`MovementComponent.StopMovementImmediately` (`self.CharacterMovement`))
        (set `CharacterMovementComponent.MaxWalkSpeed` 600.0 (`self.CharacterMovement`))
        (set `self.MoveToNewHidingLoc` true)))
    (elif (`self.PlayerDetected`)
      (bind _targetplayer_2 (`self.GetNearestPlayer` true "NewEnumerator0"))
      (bind _output_get (set `self.DetectedPlayer` _targetplayer_2))
      (bind _outhit (`KismetSystemLibrary.LineTraceSingle` (`SceneComponent.K2_GetComponentLocation` (`self.Eyes`)) (`self.GetLocation` _output_get) "TraceTypeQuery1" false (`|MakeArray` self :!type "Actor Object Reference")))
      (if (`GameplayStatics.BreakHitResult` _outhit)
        (cast `/Game/Framework/Blueprints/AI/BP_Player` (`.HitActor` (`GameplayStatics.BreakHitResult` _outhit)))
        (`self.UpdateEQS`))
      (else
        (`MovementComponent.StopMovementImmediately` (`self.CharacterMovement`))
        (set `CharacterMovementComponent.MaxWalkSpeed` 600.0 (`self.CharacterMovement`))
        (set `self.MoveToNewHidingLoc` true)))))

(event `self.DetectionTrigger.OnComponentBeginOverlap`
  (params (OverlappedComponent :type "PrimitiveComponent Object Reference") (OtherActor :type "Actor Object Reference") (OtherComp :type "PrimitiveComponent Object Reference") (OtherBodyIndex :type Integer) (bFromSweep :type Boolean) (SweepResult :type "HitResult Structure (by ref)"))
  (bind _asbp_player (cast `/Game/Framework/Blueprints/AI/BP_Player` OtherActor))
  (set `self.UseSight` false)
  (`self.PlayerSensed` "NewEnumerator0" _asbp_player))

(event `self.DetectionTrigger.OnComponentEndOverlap`
  (params (OverlappedComponent :type "PrimitiveComponent Object Reference") (OtherActor :type "Actor Object Reference") (OtherComp :type "PrimitiveComponent Object Reference") (OtherBodyIndex :type Integer))
  (bind _asbp_player (cast `/Game/Framework/Blueprints/AI/BP_Player` OtherActor))
  (set `self.UseSight` true)
  (`self.PlayerUnsensed` "NewEnumerator0" _asbp_player))

(event `self.SightTrigger.OnComponentBeginOverlap`
  (params (OverlappedComponent :type "PrimitiveComponent Object Reference") (OtherActor :type "Actor Object Reference") (OtherComp :type "PrimitiveComponent Object Reference") (OtherBodyIndex :type Integer) (bFromSweep :type Boolean) (SweepResult :type "HitResult Structure (by ref)"))
  (bind _asbp_player (cast `/Game/Framework/Blueprints/AI/BP_Player` OtherActor))
  (`self.PlayerSensed` "NewEnumerator1" _asbp_player))

(event `self.SightTrigger.OnComponentEndOverlap`
  (params (OverlappedComponent :type "PrimitiveComponent Object Reference") (OtherActor :type "Actor Object Reference") (OtherComp :type "PrimitiveComponent Object Reference") (OtherBodyIndex :type Integer))
  (bind _asbp_player (cast `/Game/Framework/Blueprints/AI/BP_Player` OtherActor))
  (`self.PlayerUnsensed` "NewEnumerator1" _asbp_player))

(event `self.NearWallTrigger.OnComponentEndOverlap`
  (params (OverlappedComponent :type "PrimitiveComponent Object Reference") (OtherActor :type "Actor Object Reference") (OtherComp :type "PrimitiveComponent Object Reference") (OtherBodyIndex :type Integer))
  (cast `StaticMeshActor` OtherActor)
  (set `self.NearWall` false))

(event `self.NearWallTrigger.OnComponentBeginOverlap`
  (params (OverlappedComponent :type "PrimitiveComponent Object Reference") (OtherActor :type "Actor Object Reference") (OtherComp :type "PrimitiveComponent Object Reference") (OtherBodyIndex :type Integer) (bFromSweep :type Boolean) (SweepResult :type "HitResult Structure (by ref)"))
  (cast `StaticMeshActor` OtherActor)
  (set `self.NearWall` true))

(event `Wander`
  (set `self.IsChasingAPlayer` false)
  (if (`self.NearWall`)
    (`/Game/Framework/Core/Libraries/BPML_General.MoveToRandomLocation` self (`SceneComponent.K2_GetComponentLocation` (`self.WanderLocBehind`)) 48.0 true 1000.0)
    (else
      (`/Game/Framework/Core/Libraries/BPML_General.MoveToRandomLocation` self (`SceneComponent.K2_GetComponentLocation` (`self.WanderLoc`)) 48.0 true 1000.0))))

(event `self.ReceiveBeginPlay`
  (bind _returnvalue (`EnvQueryManager.RunEQSQuery` "/Game/Framework/Blueprints/AI/EQS_HideFromPlayer.EQS_HideFromPlayer" self "AllMatching" "/Script/AIModule.EnvQueryInstanceBlueprintWrapper" :!label _label))
  (add `EnvQueryInstanceBlueprintWrapper.OnQueryFinishedEvent` _returnvalue (delegate `OnQueryFinishedEvent_Event_0`)))

(event `UpdateEQS`
  (goto _label))

(event `OnQueryFinishedEvent_Event_0`
  (params (QueryInstance :type "EnvQueryInstanceBlueprintWrapper Object Reference") (QueryStatus :type "EEnvQueryStatus Enum" :default "Processing"))
  (bind _resultlocations (`EnvQueryInstanceBlueprintWrapper.GetQueryResultsAsLocations` QueryInstance))
  (set `CharacterMovementComponent.MaxWalkSpeed` 1500.0 (`self.CharacterMovement`))
  (`|AIMoveTo` self (`|GetArrayItem` _resultlocations) null 10.0))

(fn `SimpleKillPlayer`
  (`KismetArrayLibrary.Array_RemoveItem` (`self.SeenPlayers`) (`self.SeenPlayer`))
  (set `self.PlayerDetected` false)
  (`self.Respawn` (`self.SeenPlayer`)))

(fn `UserConstructionScript`
  (`parent.UserConstructionScript`)
  (`SceneComponent.SetVisibility` (`self.SightWireFrame`) (`self.DebugVisible`) false)
  (`SceneComponent.SetVisibility` (`self.SightTrigger`) (`self.DebugVisible`) false)
  (`SceneComponent.SetVisibility` (`self.DetectionTrigger`) (`self.DebugVisible`) false)
  (`SceneComponent.SetVisibility` (`self.DetectionWireFrame`) (`self.DebugVisible`) false)
  ;[1 1 1] Update the wireframe mesh to match the detection trigger
  (`StaticMeshComponent.SetStaticMesh` (`self.SightWireFrame`) (`StaticMeshComponent.StaticMesh` (`self.SightTrigger`)))
  (`StaticMeshComponent.SetStaticMesh` (`self.DetectionWireFrame`) (`StaticMeshComponent.StaticMesh` (`self.DetectionTrigger`))))