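; Simple zombie AI that chases players entering its detection trigger and respawns the one it reaches.
; SRunBehavior moves to the player from GetNearestPlayer using senses, or wanders randomly when none is detected.
; Trigger overlaps maintain the detected player list and flags, and the construction script matches a debug wireframe to the trigger mesh.
; GetNearestDetectedPlayer ranks listed players by nav path cost but is not called here.
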(event `self.S_RunBehavior`
  (bind _detectedplayer (`self.DetectedPlayer`))
  (if (`self.PlayerDetected`)
    (bind _targetplayer (`self.GetNearestPlayer` true "NewEnumerator0"))
    (set `self.DetectedPlayer` _targetplayer)
    (bind _detectedplayer_2 (`self.DetectedPlayer`)
      (:`then`
        (`|AIMoveTo` self (0.0 0.0 0.0) _detectedplayer_2 40.0
          (:`OnSuccess`
            ;[1 1 1] Kill Player
            (`KismetArrayLibrary.Array_RemoveItem` (`self.DetectedPlayers`) _detectedplayer)
            (if (== _detectedplayer (`self.DetectedPlayer`))
              (set `self.PlayerDetected` false)
              (`self.Respawn` (`self.DetectedPlayer`))))))
      (:`else`
        (set `self.PlayerDetected` false)))
    (else
      (set `self.PlayerDetected` false)
      (`/Game/Framework/Core/Libraries/BPML_General.MoveToRandomLocation` self (`self.GetLocation`) 48.0 true 1000.0))))

(event `self.DetectionTrigger.OnComponentBeginOverlap`
  (params (OverlappedComponent :type "PrimitiveComponent Object Reference") (OtherActor :type "Actor Object Reference") (OtherComp :type "PrimitiveComponent Object Reference") (OtherBodyIndex :type Integer) (bFromSweep :type Boolean) (SweepResult :type "HitResult Structure (by ref)"))
  ;[1 1 1] Detection
  (bind _asbp_player (cast `/Game/Framework/Blueprints/AI/BP_Player` OtherActor))
  (if (`self.IsChasingAPlayer`)
    (bind _output_get (set `self.NewPlayer` _asbp_player))
    (`KismetArrayLibrary.Array_Add` (`self.DetectedPlayers`) _output_get)
    (else
      (bind _output_get_2 (set `self.DetectedPlayer` _asbp_player))
      (`KismetArrayLibrary.Array_Add` (`self.DetectedPlayers`) _output_get_2)
      (set `self.PlayerDetected` true)
      (set `self.IsChasingAPlayer` true))))

(event `self.DetectionTrigger.OnComponentEndOverlap`
  (params (OverlappedComponent :type "PrimitiveComponent Object Reference") (OtherActor :type "Actor Object Reference") (OtherComp :type "PrimitiveComponent Object Reference") (OtherBodyIndex :type Integer))
  ;[1 1 1] Detection
  (bind _asbp_player (cast `/Game/Framework/Blueprints/AI/BP_Player` OtherActor))
  (`KismetArrayLibrary.Array_RemoveItem` (`self.DetectedPlayers`) _asbp_player)
  (if (== _asbp_player (`self.DetectedPlayer`))
    (set `self.PlayerDetected` false)))

(fn `GetNearestDetectedPlayer`
  (returns (TargetPlayer :type "/Game/Framework/Blueprints/AI/BP_Player Object Reference"))
  (locals (L_TargetPlayer :type "Array of /Game/Framework/Blueprints/AI/BP_Player Object Reference") (L_TargetPlayerDistance :type "Array of Float (double-precision)"))
  (`KismetArrayLibrary.Array_Clear` (`local.L_TargetPlayer`))
  (`KismetArrayLibrary.Array_Clear` (`local.L_TargetPlayerDistance`))
  (for _array_element (`self.DetectedPlayers`)
    (`KismetArrayLibrary.Array_Add` (`local.L_TargetPlayer`) _array_element)
    (`KismetArrayLibrary.Array_Add` (`local.L_TargetPlayerDistance`) (`NavigationSystemV1.GetPathCost` (`self.GetLocation`) (`self.GetLocation` _array_element) null "/Script/NavigationSystem.NavigationQueryFilter")))
  (return (`|GetArrayItem` (`local.L_TargetPlayer`) (`KismetMathLibrary.MinOfFloatArray` (`local.L_TargetPlayerDistance`)))))

(fn `UserConstructionScript`
  (`parent.UserConstructionScript`)
  (`SceneComponent.SetHiddenInGame` (`self.DetectionTrigger`) (`self.DebugHiddenInGame`) false)
  (`SceneComponent.SetHiddenInGame` (`self.WireFrameMesh`) (`self.DebugHiddenInGame`) false)
  ;[1 1 1] Update the wireframe mesh to match the detection trigger
  (`StaticMeshComponent.SetStaticMesh` (`self.WireFrameMesh`) (`StaticMeshComponent.StaticMesh` (`self.DetectionTrigger`))))