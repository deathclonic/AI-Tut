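; Experimental arena bot AI pawn with player sensing, random wandering and EQS-driven hiding from players.
; Sight and detection trigger overlaps register players, while a wall trigger picks the wander origin; construction syncs debug wireframes to the sense triggers.
; UpdateEQS sprints to the first hide-query result.
; The behavior event is empty, and the sense-to-hide, waypoint roaming, strafing and scored task-selection experiments in the event graph are disconnected.
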(event `self.DetectionTrigger.OnComponentBeginOverlap`
  (params (OverlappedComponent :type "PrimitiveComponent Object Reference") (OtherActor :type "Actor Object Reference") (OtherComp :type "PrimitiveComponent Object Reference") (OtherBodyIndex :type Integer) (bFromSweep :type Boolean) (SweepResult :type "HitResult Structure (by ref)"))
  (bind _asbp_player (cast `/Game/Framework/Blueprints/AI/BP_Player` OtherActor))
  (set `self.UseSight` false)
  (`self.PlayerSensed` "NewEnumerator0" _asbp_player))

(event `self.DetectionTrigger.OnComponentEndOverlap`
  (params (OverlappedComponent :type "PrimitiveComponent Object Reference") (OtherActor :type "Actor Object Reference") (OtherComp :type "PrimitiveComponent Object Reference") (OtherBodyIndex :type Integer))
  (bind _asbp_player (cast `/Game/Framework/Blueprints/AI/BP_Player` OtherActor))
  (set `self.UseSight` true)
  (`self.PlayerUnsensed` "NewEnumerator0" _asbp_player))

(event `self.SightTrigger.OnComponentBeginOverlap`
  (params (OverlappedComponent :type "PrimitiveComponent Object Reference") (OtherActor :type "Actor Object Reference") (OtherComp :type "PrimitiveComponent Object Reference") (OtherBodyIndex :type Integer) (bFromSweep :type Boolean) (SweepResult :type "HitResult Structure (by ref)"))
  (bind _asbp_player (cast `/Game/Framework/Blueprints/AI/BP_Player` OtherActor))
  (`self.PlayerSensed` "NewEnumerator1" _asbp_player))

(event `self.SightTrigger.OnComponentEndOverlap`
  (params (OverlappedComponent :type "PrimitiveComponent Object Reference") (OtherActor :type "Actor Object Reference") (OtherComp :type "PrimitiveComponent Object Reference") (OtherBodyIndex :type Integer))
  (bind _asbp_player (cast `/Game/Framework/Blueprints/AI/BP_Player` OtherActor))
  (`self.PlayerUnsensed` "NewEnumerator1" _asbp_player))

(event `self.NearWallTrigger.OnComponentEndOverlap`
  (params (OverlappedComponent :type "PrimitiveComponent Object Reference") (OtherActor :type "Actor Object Reference") (OtherComp :type "PrimitiveComponent Object Reference") (OtherBodyIndex :type Integer))
  (cast `StaticMeshActor` OtherActor)
  (set `self.NearWall` false))

(event `self.NearWallTrigger.OnComponentBeginOverlap`
  (params (OverlappedComponent :type "PrimitiveComponent Object Reference") (OtherActor :type "Actor Object Reference") (OtherComp :type "PrimitiveComponent Object Reference") (OtherBodyIndex :type Integer) (bFromSweep :type Boolean) (SweepResult :type "HitResult Structure (by ref)"))
  (cast `StaticMeshActor` OtherActor)
  (set `self.NearWall` true))

(event `Wander`
  (set `self.IsChasingAPlayer` false)
  (if (`self.NearWall`)
    (`/Game/Framework/Core/Libraries/BPML_General.MoveToRandomLocation` self (`SceneComponent.K2_GetComponentLocation` (`self.WanderLocBehind`)) 48.0 true 1000.0)
    (else
      (`/Game/Framework/Core/Libraries/BPML_General.MoveToRandomLocation` self (`SceneComponent.K2_GetComponentLocation` (`self.WanderLoc`)) 48.0 true 1000.0))))

(event `UpdateEQS`
  (bind _returnvalue (`EnvQueryManager.RunEQSQuery` "/Game/Framework/Blueprints/AI/EQS_HideFromPlayer.EQS_HideFromPlayer" self "AllMatching" "/Script/AIModule.EnvQueryInstanceBlueprintWrapper"))
  (add `EnvQueryInstanceBlueprintWrapper.OnQueryFinishedEvent` _returnvalue (delegate `OnQueryFinishedEvent_Event_0`)))

(event `self.ReceiveBeginPlay`
  (bind _outactors (`GameplayStatics.GetAllActorsOfClass` "/Game/Framework/Blueprints/AI/FuzzyAI/BP_AiWaypoint.BP_AiWaypoint_C"))
  (set `self.Waypoints` _outactors)
  (bind _asbp_core_aic (cast `/Game/Framework/Core/BP_CoreAIC` (`AIBlueprintHelperLibrary.GetAIController` self)))
  (set `self.AiController` _asbp_core_aic))

(event `OnQueryFinishedEvent_Event_0`
  (params (QueryInstance :type "EnvQueryInstanceBlueprintWrapper Object Reference") (QueryStatus :type "EEnvQueryStatus Enum" :default "Processing"))
  (bind _resultlocations (`EnvQueryInstanceBlueprintWrapper.GetQueryResultsAsLocations` QueryInstance))
  (set `CharacterMovementComponent.MaxWalkSpeed` 1500.0 (`self.CharacterMovement`))
  (`|AIMoveTo` self (`|GetArrayItem` _resultlocations) null 10.0))

(event `self.S_RunBehavior`)

(fn `ScoreTask`
  (params (`Task ID` :type Name) (Score :type "Float (double-precision)"))
  (returns (Task :type "/Game/Framework/Blueprints/AI/S_Task Structure"))
  (return (make `/Game/Framework/Blueprints/AI/S_Task` `Task ID` Score (`self.TargetActor`))))

(fn `SelectTask`
  (params (Tasks :type "Array of /Game/Framework/Blueprints/AI/S_Task Structure") (Selection :type "/Game/Framework/Blueprints/AI/E_SelectionMode Enum" :default "NewEnumerator0"))
  (returns (Selected :type "/Game/Framework/Blueprints/AI/S_Task Structure"))
  (locals (HighestScoredTaskID :type Name) (SelectedTask :type "/Game/Framework/Blueprints/AI/S_Task Structure") (HighestScore :type "Float (double-precision)" :default 0.0))
  (for _array_element Tasks
    (if (> (`.Score_7_6F34317B41E70906BB0465AC71AFE29C` (break `/Game/Framework/Blueprints/AI/S_Task` _array_element)) (`local.HighestScore`))
      (set `local.SelectedTask` _array_element)))
  (return (`local.SelectedTask`)))

(fn `SimpleKillPlayer`
  (`KismetArrayLibrary.Array_RemoveItem` (`self.SeenPlayers`) (`self.SeenPlayer`))
  (set `self.PlayerDetected` false)
  (`self.Respawn` (`self.SeenPlayer`)))

(fn `UserConstructionScript`
  (`parent.UserConstructionScript`)
  (`SceneComponent.SetVisibility` (`self.SightWireFrame`) (`self.DebugVisible`) false)
  (`SceneComponent.SetVisibility` (`self.SightTrigger`) (`self.DebugVisible`) false)
  (`SceneComponent.SetVisibility` (`self.DetectionTrigger`) (`self.DebugVisible`) false)
  (`SceneComponent.SetVisibility` (`self.DetectionWireFrame`) (`self.DebugVisible`) false)
  ;[1 1 1] Update the wireframe mesh to match the detection trigger
  (`StaticMeshComponent.SetStaticMesh` (`self.SightWireFrame`) (`StaticMeshComponent.StaticMesh` (`self.SightTrigger`)))
  (`StaticMeshComponent.SetStaticMesh` (`self.DetectionWireFrame`) (`StaticMeshComponent.StaticMesh` (`self.DetectionTrigger`))))