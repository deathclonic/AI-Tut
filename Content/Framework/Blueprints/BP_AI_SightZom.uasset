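; Child AI Blueprint for a sight-based zombie that wanders, chases players and respawns SeenPlayer on reaching its target.
; Sight and detection mesh triggers report players to inherited sensing, with detection overlap switching off sight logic.
; SRunBehavior chases the nearest sensed player, investigates the last seen location, or wanders.
; Wandering picks random points around a WanderLoc component, using the one behind when NearWallTrigger overlaps a static mesh actor.
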(event `self.S_RunBehavior`
  (if (`self.UseSight`)
    (bind _targetplayer (`self.GetNearestPlayer` true "NewEnumerator1"))
    (set `self.SeenPlayer` _targetplayer)
    (`self.SightPerception`)
    (if (`self.PlayerCurrentlyInSight`)
      ;[1 1 1] Move to seen player
      (bind _seenplayer (`self.SeenPlayer`)
        (:`then`
          (`|AIMoveTo` self (0.0 0.0 0.0) _seenplayer 40.0
            (:`OnSuccess`
              (`self.SimpleKillPlayer`))))
        (:`else`
          (set `self.PlayerCurrentlyInSight` false)))
      (elif (`self.bPlayerSeen`)
        ;[1 1 1] Move to last seen location
        (`|AIMoveTo` self (`self.LastSeenLocation`) null 40.0 true
          (:`OnSuccess`
            (set `self.bPlayerSeen` false)))
        (else
          (`self.Wander`))))
    (elif (`self.PlayerDetected`)
      (bind _targetplayer_2 (`self.GetNearestPlayer` true "NewEnumerator0"))
      (set `self.DetectedPlayer` _targetplayer_2)
      (bind _detectedplayer (`self.DetectedPlayer`)
        (:`then`
          (`|AIMoveTo` self (0.0 0.0 0.0) _detectedplayer 40.0
            (:`OnSuccess`
              (`self.SimpleKillPlayer`))))
        (:`else`
          (set `self.PlayerDetected` false)))
      (else
        (set `self.PlayerDetected` false)
        (`self.Wander`)))))

(event `self.DetectionTrigger.OnComponentBeginOverlap`
  (params (OverlappedComponent :type "PrimitiveComponent Object Reference") (OtherActor :type "Actor Object Reference") (OtherComp :type "PrimitiveComponent Object Reference") (OtherBodyIndex :type Integer) (bFromSweep :type Boolean) (SweepResult :type "HitResult Structure (by ref)"))
  (bind _asbp_player (cast `/Game/Framework/Blueprints/BP_Player` OtherActor))
  (set `self.UseSight` false)
  (`self.PlayerSensed` "NewEnumerator0" _asbp_player))

(event `self.DetectionTrigger.OnComponentEndOverlap`
  (params (OverlappedComponent :type "PrimitiveComponent Object Reference") (OtherActor :type "Actor Object Reference") (OtherComp :type "PrimitiveComponent Object Reference") (OtherBodyIndex :type Integer))
  (bind _asbp_player (cast `/Game/Framework/Blueprints/BP_Player` OtherActor))
  (set `self.UseSight` true)
  (`self.PlayerUnsensed` "NewEnumerator0" _asbp_player))

(event `self.SightTrigger.OnComponentBeginOverlap`
  (params (OverlappedComponent :type "PrimitiveComponent Object Reference") (OtherActor :type "Actor Object Reference") (OtherComp :type "PrimitiveComponent Object Reference") (OtherBodyIndex :type Integer) (bFromSweep :type Boolean) (SweepResult :type "HitResult Structure (by ref)"))
  (bind _asbp_player (cast `/Game/Framework/Blueprints/BP_Player` OtherActor))
  (`self.PlayerSensed` "NewEnumerator1" _asbp_player))

(event `self.SightTrigger.OnComponentEndOverlap`
  (params (OverlappedComponent :type "PrimitiveComponent Object Reference") (OtherActor :type "Actor Object Reference") (OtherComp :type "PrimitiveComponent Object Reference") (OtherBodyIndex :type Integer))
  (bind _asbp_player (cast `/Game/Framework/Blueprints/BP_Player` OtherActor))
  (`self.PlayerUnsensed` "NewEnumerator1" _asbp_player))

(event `self.NearWallTrigger.OnComponentEndOverlap`
  (params (OverlappedComponent :type "PrimitiveComponent Object Reference") (OtherActor :type "Actor Object Reference") (OtherComp :type "PrimitiveComponent Object Reference") (OtherBodyIndex :type Integer))
  (cast `StaticMeshActor` OtherActor)
  (set `self.NearWall` false))

(event `self.NearWallTrigger.OnComponentBeginOverlap`
  (params (OverlappedComponent :type "PrimitiveComponent Object Reference") (OtherActor :type "Actor Object Reference") (OtherComp :type "PrimitiveComponent Object Reference") (OtherBodyIndex :type Integer) (bFromSweep :type Boolean) (SweepResult :type "HitResult Structure (by ref)"))
  (cast `StaticMeshActor` OtherActor)
  (set `self.NearWall` true))

(event `Wander`
  (set `self.IsChasingAPlayer` false)
  (if (`self.NearWall`)
    (`/Game/Framework/Core/Libraries/BPML_General.MoveToRandomLocation` self (`SceneComponent.K2_GetComponentLocation` (`self.WanderLocBehind`)) 48.0 true 1000.0)
    (else
      (`/Game/Framework/Core/Libraries/BPML_General.MoveToRandomLocation` self (`SceneComponent.K2_GetComponentLocation` (`self.WanderLoc`)) 48.0 true 1000.0))))

(fn `SimpleKillPlayer`
  (`KismetArrayLibrary.Array_RemoveItem` (`self.SeenPlayers`) (`self.SeenPlayer`))
  (set `self.PlayerDetected` false)
  (`self.Respawn` (`self.SeenPlayer`)))

(fn `UserConstructionScript`
  (`parent.UserConstructionScript`)
  (`SceneComponent.SetVisibility` (`self.SightWireFrame`) (`self.DebugVisible`) false)
  (`SceneComponent.SetVisibility` (`self.SightTrigger`) (`self.DebugVisible`) false)
  (`SceneComponent.SetVisibility` (`self.DetectionTrigger`) (`self.DebugVisible`) false)
  (`SceneComponent.SetVisibility` (`self.DetectionWireFrame`) (`self.DebugVisible`) false)
  ;[1 1 1] Update the wireframe mesh to match the detection trigger
  (`StaticMeshComponent.SetStaticMesh` (`self.SightWireFrame`) (`StaticMeshComponent.StaticMesh` (`self.SightTrigger`))))